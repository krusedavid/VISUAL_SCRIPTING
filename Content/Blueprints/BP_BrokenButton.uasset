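; Interactable push button that either works or is broken, set by the BrokenButton flag.
; Interact plays a timeline that slides the mesh along Y, with the flag checked on every timeline update.
; A working button plays a sound and particles, then after a delay calls FinalButton on the first-person character and InteractMessage on Engine.
; A broken one plays a click and reveals BrokenLight.
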(event `/Game/Blueprints/BPI_Interact.Interact`
  ;[1 1 1] Moving button
  (bind (_direction _buttontrack) (`Timeline|Moving Button` :!via `PlayFromStart`)
    (:`Update`
      (`SceneComponent.K2_SetRelativeLocation` (`self.StaticMesh`) (`KismetMathLibrary.MakeVector` 0.0 (`KismetMathLibrary.Lerp` 0.0 5.0 _buttontrack)) false false)
      ;;[1 1 1] Broken Button
      (if (not (`self.BrokenButton`))
        (`GameplayStatics.PlaySound2D` "/Engine/VREditor/Sounds/UI/Gizmo_Handle_Clicked.Gizmo_Handle_Clicked" 1.0 1.0 0.0 null null)
        (`ActorComponent.Activate` (`self.ParticleSystem`) false)
        (`KismetSystemLibrary.Delay` 10.0)
        (bind _returnvalue (`GameplayStatics.GetActorOfClass` "/Game/FirstPerson/Blueprints/BP_FirstPersonCharacter.BP_FirstPersonCharacter_C"))
        (bind _asbp_first_person_character (cast `/Game/FirstPerson/Blueprints/BP_FirstPersonCharacter` _returnvalue))
        (`/Game/FirstPerson/Blueprints/BP_FirstPersonCharacter.FinalButton` _asbp_first_person_character)
        (message `/Game/Blueprints/BPI_Interact.Interact` (`self.Engine`))
        (else
          (`GameplayStatics.PlaySoundAtLocation` "/Engine/VREditor/Sounds/UI/Click_on_Button_Cue.Click_on_Button_Cue" (0.0 0.0 0.0) (struct) 1.0 1.0 0.0 null null null null)
          (`SceneComponent.SetVisibility` (`self.BrokenLight`) true false))))))

(fn `UserConstructionScript`)