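; Checkpoint actor that sets the first-person character's respawn point when the player walks into it.
; On overlap with the Checkpoint box, it passes the SpawnLocation component's world position to the character's NewSpawnLocation.
; The construction script sizes the box and positions the spawn point from the InBoxExtent and SpawnPointVector variables, so each placed instance can be tuned.
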(event `self.Checkpoint.OnComponentBeginOverlap`
  (params (OverlappedComponent :type "PrimitiveComponent Object Reference") (OtherActor :type "Actor Object Reference") (OtherComp :type "PrimitiveComponent Object Reference") (OtherBodyIndex :type Integer) (bFromSweep :type Boolean) (SweepResult :type "HitResult Structure (by ref)"))
  (bind _asbp_first_person_character (cast `/Game/FirstPerson/Blueprints/BP_FirstPersonCharacter` OtherActor))
  (`/Game/FirstPerson/Blueprints/BP_FirstPersonCharacter.NewSpawnLocation` _asbp_first_person_character (`SceneComponent.K2_GetComponentLocation` (`self.SpawnLocation`))))

(fn `UserConstructionScript`
  (`BoxComponent.SetBoxExtent` (`self.Checkpoint`) (`self.In Box Extent`) true)
  (`SceneComponent.K2_SetRelativeLocation` (`self.SpawnLocation`) (`self.SpawnPointVector`) false false))