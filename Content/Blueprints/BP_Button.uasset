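; Interactable button Blueprint that, unless flagged broken, triggers the player character's FinalButton sequence.
; Interact plays a timeline that shifts the button's relative Y, with Location.Y fed into Z.
; On each timeline update, a working button plays a click, then after a delay calls FinalButton and sends InteractMessage to Engine.
; A broken button only plays a click at the world origin; the smoke emitter node is unconnected.
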(event `/Game/Blueprints/BPI_Interact.Interact`
  ;[1 1 1] Moving button
  (bind _output_get (set `self.Location` (`SceneComponent.RelativeLocation` (`self.Button`))))
  (bind (_direction _buttontrack) (`Timeline|Moving Button` :!via `PlayFromStart`)
    (:`Update`
      (`SceneComponent.K2_SetRelativeLocation` (`self.Button`) (`KismetMathLibrary.MakeVector` (.x _output_get) (`KismetMathLibrary.Lerp` 0.0 5.0 _buttontrack) (.y _output_get)) false false)
      (if (not (`self.BrokenButton`))
        (`GameplayStatics.PlaySound2D` "/Engine/VREditor/Sounds/VR_click3_Cue.VR_click3_Cue" 1.0 1.0 0.0 null null)
        (`KismetSystemLibrary.Delay` 10.0)
        (bind _returnvalue (`GameplayStatics.GetActorOfClass` "/Game/FirstPerson/Blueprints/BP_FirstPersonCharacter.BP_FirstPersonCharacter_C"))
        (bind _asbp_first_person_character (cast `/Game/FirstPerson/Blueprints/BP_FirstPersonCharacter` _returnvalue))
        (`/Game/FirstPerson/Blueprints/BP_FirstPersonCharacter.FinalButton` _asbp_first_person_character)
        (message `/Game/Blueprints/BPI_Interact.Interact` (`self.Engine`))
        (else
          (`GameplayStatics.PlaySoundAtLocation` "/Engine/VREditor/Sounds/UI/Click_on_Button_Cue.Click_on_Button_Cue" (0.0 0.0 0.0) (struct) 1.0 1.0 0.0 null null null null))))))

(fn `UserConstructionScript`)